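; Blueprint function library of 2D math for fisheye lens distortion of UV coordinates.
; Fisheye applies aspect-corrected radial distortion normalized to the viewport diagonal, using tangent for barrel and arctangent for pinch, chosen by the sign of Angle.
; Separate helpers, not called by Fisheye, compute spherical radial gradients with inverse variants, lerp 2D vectors, and mirror coordinates around the UV center or undo that mirror.
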(fn SphereGradient2D
  (params (UVs :type Vector%202D%20Structure) (CenterPosition :type Vector%202D%20Structure :default "(X=0.500000,Y=0.500000)") (Radius :type Float%20%28double-precision%29))
  (LocalVariables|SetMyRadius Radius)
  (return (Math|Float|Clamp(Float) (/ (Math|Float|Sqrt (Math|Float|Max(Float) (- (* (LocalVariables|GetMyRadius) (LocalVariables|GetMyRadius)) (* (Math|Float|Clamp(Float) (Math|Vector|Distance2D(Vector) UVs CenterPosition) 0.0 (LocalVariables|GetMyRadius)) (Math|Float|Clamp(Float) (Math|Vector|Distance2D(Vector) UVs CenterPosition) 0.0 (LocalVariables|GetMyRadius)))) 0.0)) (LocalVariables|GetMyRadius))) (- 1.0 (Math|Trig|Cos(Radians) (Class|KismetMathLibrary|Asin (- 1.0 (/ (Math|Float|Clamp(Float) (Math|Vector|Distance2D(Vector) UVs CenterPosition) 0.0 (LocalVariables|GetMyRadius)) (LocalVariables|GetMyRadius))))))))

(fn LerpVector2D
  (params (A :type Vector%202D%20Structure) (B :type Vector%202D%20Structure) (Alpha :type Float%20%28double-precision%29))
  (bind (_x _y) (Math|Vector2D|BreakVector2D A))
  (bind (_x_2 _y_2) (Math|Vector2D|BreakVector2D B))
  (return (Math|Vector2D|MakeVector2D (Math|Float|Lerp _x _x_2 Alpha) (Math|Float|Lerp _y _y_2 Alpha))))

(fn ReverseSphereGradient2D
  (params (UVs :type Vector%202D%20Structure) (CenterPosition :type Vector%202D%20Structure :default "(X=0.500000,Y=0.500000)") (Radius :type Float%20%28double-precision%29))
  (LocalVariables|SetMyRadius Radius)
  (return (- 1.0 (Math|Trig|Cos(Radians) (Class|KismetMathLibrary|Asin (- 1.0 (/ (Math|Float|Clamp(Float) (Math|Vector|Distance2D(Vector) UVs CenterPosition) 0.0 (LocalVariables|GetMyRadius)) (LocalVariables|GetMyRadius)))))) (Math|Trig|Sin(Radians) (Math|Trig|Acos(Degrees) (/ (Math|Float|Clamp(Float) (Math|Vector|Distance2D(Vector) UVs CenterPosition) 0.0 (LocalVariables|GetMyRadius)) (LocalVariables|GetMyRadius)))) (Math|Trig|Cos(Radians) (Class|KismetMathLibrary|Asin (/ (Math|Float|Clamp(Float) (Math|Vector|Distance2D(Vector) UVs CenterPosition) 0.0 (LocalVariables|GetMyRadius)) (LocalVariables|GetMyRadius))))))

(fn MirrorVector2D
  (params (A :type Vector%202D%20Structure) (Alpha :type Float%20%28double-precision%29))
  (bind (_x _y) (Math|Vector2D|BreakVector2D A))
  (bind _returnvalue (- "(X=1.000000,Y=1.000000)" A))
  (bind (_x_2 _y_2) (Math|Vector2D|BreakVector2D _returnvalue))
  (return (Math|Vector2D|MakeVector2D (Math|Float|Lerp _x _x_2 Alpha) (Math|Float|Lerp _y _y_2 Alpha))))

(fn ReverseMirrorVector2D
  (params (A :type Vector%202D%20Structure) (Alpha :type Float%20%28double-precision%29))
  (return (- "(X=1.000000,Y=1.000000)" (/ (- (+ A Alpha) 1.0) (- (* Alpha 2.0) 1.0)))))

(fn Fisheye
  (params (UV :type Vector%202D%20Structure) (ViewSize :type Vector%202D%20Structure :default "(X=1.000000,Y=1.000000)") (angle :type Float%20%28double-precision%29))
  (bind _returnvalue (Math|Float|Absolute(Float) angle))
  (bind (_x _y) (Math|Vector2D|BreakVector2D ViewSize))
  (bind _returnvalue_2 (* UV 2.0))
  (bind _returnvalue_3 (/ _x _y))
  (bind _returnvalue_4 (/ _returnvalue 2.0))
  (bind _returnvalue_5 (- _returnvalue_2 1.0))
  (bind _returnvalue_6 (Math|Vector2D|MakeVector2D _returnvalue_3 1.0))
  (bind _returnvalue_7 (Math|Trig|Tan(Radians) _returnvalue_4))
  (bind _returnvalue_8 (Math|Vector2D|Normalize2D _returnvalue_6))
  (bind _returnvalue_9 (Math|Vector2D|Vector2DLength _returnvalue_6))
  (bind _returnvalue_10 (* _returnvalue_5 _returnvalue_6))
  (bind _returnvalue_11 (Math|Vector2D|Normalize2D _returnvalue_10))
  (bind _returnvalue_12 (Math|Vector2D|Vector2DLength _returnvalue_10))
  (bind _returnvalue_13 (/ _returnvalue_12 _returnvalue_9))
  (bind _returnvalue_14 (/ _returnvalue_11 _returnvalue_8))
  (return (+ (* (select (< angle 0.0) (/ (* _returnvalue_14 (Math|Trig|Atan(Degrees) (* _returnvalue_13 _returnvalue_7))) _returnvalue_4) (/ (* _returnvalue_14 (Math|Trig|Tan(Radians) (* _returnvalue_13 _returnvalue_4))) _returnvalue_7)) 0.5) 0.5)))